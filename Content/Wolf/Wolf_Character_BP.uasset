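; Wolf character Blueprint that patrols a looping route through a list of target points.
; On BeginPlay it issues an AI MoveTo toward the current entry in the TargetPoints array.
; Each successful arrival advances the index, wrapping to the first point after the last, and starts the next move.
; Failed moves are not handled, so the patrol stops if one fails.
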(event EventBeginPlay
  (AI|AIMoveTo self "0, 0, 0" (Utilities|Array|Get(acopy) (Variables|Default|GetTargetPoints) (Variables|Default|GetTargetPointIndex)) 5.0 false :!label _label
    (:OnSuccess
      (if (>= (Variables|Default|GetTargetPointIndex) (- (Utilities|Array|Length (Variables|Default|GetTargetPoints)) 1))
        (Variables|Default|SetTargetPointIndex 0)
        (goto _label)
        (else
          (Math|Integer|IncrementInt (Variables|Default|GetTargetPointIndex)
            (:%20%20
              (goto _label))))))))

(fn ConstructionScript)