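; SpawnVolume is an island map actor that spawns a random batch of enemies inside its Volume box when play begins.
; SpawnInterval runs once without a timer, picking a count between MinEnemies and MaxEnemies and a random ItemsToSpawn class for each spawn.
; Each actor gets a random point in the box, with collision adjusted but spawning guaranteed.
; EnemiesAppeared records the count, which is then printed, and RandomMultipleObjects is an empty stub.
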(event EventBeginPlay
  (CallFunction|SpawnInterval)
  (Development|PrintString (Utilities|String|ToString(Integer) (Variables|Default|GetEnemiesAppeared))))

(fn ConstructionScript)

(fn SpawnInterval
  (bind _volume (Variables|Default|GetVolume))
  (for _index (range 1 (Math|Random|RandomIntegerinRange (Variables|Default|GetMin%20Enemies) (Variables|Default|GetMax%20enemies)))
    (Game|SpawnActorfromClass (Utilities|Array|Get(acopy) (Variables|Default|GetItemsToSpawn) (Math|Random|RandomIntegerinRange 0 (- (Utilities|Array|Length (Variables|Default|GetItemsToSpawn)) 1))) (Math|Conversions|ToTransform(Vector) (Math|Random|RandomPointinBoundingBox (Transformation|GetWorldLocation _volume) (Components|Box|GetScaledBoxExtent _volume))) "AdjustIfPossibleButAlwaysSpawn" 0 0)
    (Variables|Default|SetEnemiesAppeared _index)))

(fn RandomMultipleObjects)